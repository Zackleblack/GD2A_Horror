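; BP_Screwdriver is a screwdriver pickup that the main character collects through interaction.
; On BeginPlay it caches a reference to the player character and creates a WBP_Interact prompt widget.
; Box overlap begin and end show and hide that prompt for the main character.
; The Interact event calls ScrewDriverPickup on the cached character, then destroys the actor.
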(event `self.ReceiveBeginPlay`
  (`|ExecutionSequence`
    (:`then_0`
      (bind _asbp_main_character (cast `/Game/FirstPerson/MainCharacter/BP_MainCharacter` (`GameplayStatics.GetPlayerCharacter` 0)))
      (set `self.Main Character Reference` _asbp_main_character))
    (:`then_1`
      (bind _returnvalue (`|CreateWidget` "/Game/DevFolder/Widgets/WBP_Interact.WBP_Interact_C"))
      (set `self.Interact widget Reference` _returnvalue))))

(event `/Game/FirstPerson/MainCharacter/BPI_Interact.Interact`
  (`/Game/FirstPerson/MainCharacter/BP_MainCharacter.Screw Driver Pickup` (`self.Main Character Reference`))
  (`self.K2_DestroyActor`))

(event `self.Box.OnComponentBeginOverlap`
  (params (OverlappedComponent :type "PrimitiveComponent Object Reference") (OtherActor :type "Actor Object Reference") (OtherComp :type "PrimitiveComponent Object Reference") (OtherBodyIndex :type Integer) (bFromSweep :type Boolean) (SweepResult :type "HitResult Structure (by ref)"))
  (cast `/Game/FirstPerson/MainCharacter/BP_MainCharacter` OtherActor)
  (`UserWidget.AddToViewport` (`self.Interact widget Reference`) 0))

(event `self.Box.OnComponentEndOverlap`
  (params (OverlappedComponent :type "PrimitiveComponent Object Reference") (OtherActor :type "Actor Object Reference") (OtherComp :type "PrimitiveComponent Object Reference") (OtherBodyIndex :type Integer))
  (cast `/Game/FirstPerson/MainCharacter/BP_MainCharacter` OtherActor)
  (`Widget.RemoveFromParent` (`self.Interact widget Reference`)))

(fn `UserConstructionScript`)