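; Key-locked swinging door that the main character opens and closes through Interact once PickUpKey has set HasKey.
; A FlipFlop plays or reverses DoorTimeline, which lerps the mesh yaw and disables its collision until the swing finishes.
; A DoOnce, reset on finish, limits the door sound to once per swing.
; Leaving the collision volume reverses an open door after delays, while entering only prints a debug message.
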(event `self.ReceiveBeginPlay`
  (bind _asbp_main_character (cast `/Game/FirstPerson/MainCharacter/BP_MainCharacter` (`GameplayStatics.GetPlayerCharacter` 0)))
  (set `self.Main Character Reference` _asbp_main_character))

(event `self.Player Collision.OnComponentBeginOverlap`
  (params (OverlappedComponent :type "PrimitiveComponent Object Reference") (OtherActor :type "Actor Object Reference") (OtherComp :type "PrimitiveComponent Object Reference") (OtherBodyIndex :type Integer) (bFromSweep :type Boolean) (SweepResult :type "HitResult Structure (by ref)"))
  (cast `/Game/FirstPerson/MainCharacter/BP_MainCharacter` OtherActor)
  (`KismetSystemLibrary.PrintString` "You are in front of Door")
  (if true
    _))

(event `/Game/FirstPerson/MainCharacter/BPI_Interact.Interact`
  (bind _sm_door (`self.SM_Door`))
  (if (`self.bHasKey?`)
    (`/Engine/EditorBlueprintResources/StandardMacros.FlipFlop`
      (:`A`
        (bind (_direction _opening_door) (`Timeline|Door timeline` :!label _label)
          (:`Update`
            (`|ExecutionSequence`
              (:`then_0`
                (`/Engine/EditorBlueprintResources/StandardMacros.DoOnce` false :!label _label_2
                  (:`Completed`
                    (`GameplayStatics.PlaySoundAtLocation` "/Game/DevFolder/Blueprints/Door/Door_Open_Cue.Door_Open_Cue" (`SceneComponent.K2_GetComponentLocation` (`self.SM_Door`)) (struct) 1.0 1.0 0.0 null null null null))))
              (:`then_1`
                (set `self.bIsDoorOpen?` true)
                (`PrimitiveComponent.SetCollisionEnabled` _sm_door "NoCollision")
                (`SceneComponent.K2_SetRelativeRotation` _sm_door (`KismetMathLibrary.MakeRotator` 0.0 0.0 (`KismetMathLibrary.Lerp` 0.0 120.0 _opening_door)) false false))))
          (:`Finished`
            (`|ExecutionSequence`
              (:`then_0`
                (goto _label_2 :!via `Reset`))
              (:`then_1`
                (`PrimitiveComponent.SetCollisionEnabled` _sm_door "QueryAndPhysics"))))))
      (:`B`
        (set `self.bIsDoorOpen?` false)
        (goto _label :!via `Reverse`)))))

(event `/Game/DevFolder/Blueprints/Door/BPI_Door.Pick Up Key`
  (set `self.bHasKey?` true))

(event `self.Player Collision.OnComponentEndOverlap`
  (params (OverlappedComponent :type "PrimitiveComponent Object Reference") (OtherActor :type "Actor Object Reference") (OtherComp :type "PrimitiveComponent Object Reference") (OtherBodyIndex :type Integer))
  (cast `/Game/FirstPerson/MainCharacter/BP_MainCharacter` OtherActor)
  (`KismetSystemLibrary.Delay` 5.0)
  (if (`self.bIsDoorOpen?`)
    (`KismetSystemLibrary.Delay` 5.0)
    (goto _label :!via `Reverse`)))

(fn `UserConstructionScript`)