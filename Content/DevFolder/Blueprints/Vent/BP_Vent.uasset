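; BP_Vent is an interactable vent that the player can move aside only after picking up a screwdriver.
; Interact checks the main character's screwdriver flag, then a one-shot timeline lerps the vent mesh toward the GoToVent component's relative location, with VentMoved blocking repeats.
; A collision overlap tracks whether the main character is in front of the vent, and debug prints report each state.
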(event `self.ReceiveBeginPlay`)

(event `self.Vent Collision.OnComponentBeginOverlap`
  (params (OverlappedComponent :type "PrimitiveComponent Object Reference") (OtherActor :type "Actor Object Reference") (OtherComp :type "PrimitiveComponent Object Reference") (OtherBodyIndex :type Integer) (bFromSweep :type Boolean) (SweepResult :type "HitResult Structure (by ref)"))
  (cast `/Game/FirstPerson/MainCharacter/BP_MainCharacter` OtherActor)
  (set `self.bInFrontOfVent?` true)
  (`KismetSystemLibrary.PrintString` "You Are In Front of Vent"))

(event `self.Vent Collision.OnComponentEndOverlap`
  (params (OverlappedComponent :type "PrimitiveComponent Object Reference") (OtherActor :type "Actor Object Reference") (OtherComp :type "PrimitiveComponent Object Reference") (OtherBodyIndex :type Integer))
  (cast `/Game/FirstPerson/MainCharacter/BP_MainCharacter` OtherActor)
  (set `self.bInFrontOfVent?` false)
  (`KismetSystemLibrary.PrintString` "You Are No Longer in Front of Vent"))

(event `/Game/FirstPerson/MainCharacter/BPI_Interact.Interact`
  (bind _vent (`self.Vent`))
  (if (`self.bVentMoved?`)
    (`KismetSystemLibrary.PrintString` "The Vent has already been moved")
    (else
      (bind _asbp_main_character (cast `/Game/FirstPerson/MainCharacter/BP_MainCharacter` (`GameplayStatics.GetPlayerCharacter` 0)))
      (if (`/Game/FirstPerson/MainCharacter/BP_MainCharacter.bPickUpScrewdriver?` _asbp_main_character)
        (set `self.bVentMoved?` true)
        (bind (_direction _vent_move_animation) (`Timeline|Vent Timeline`)
          (:`Update`
            (`SceneComponent.K2_SetRelativeLocation` _vent (`KismetMathLibrary.VLerp` (`SceneComponent.RelativeLocation` _vent) (`SceneComponent.RelativeLocation` (`self.GoToVent`)) _vent_move_animation) false false)))
        (else
          (`KismetSystemLibrary.PrintString` "You need a screw driver to open this..."))))))

(fn `UserConstructionScript`)