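; BP_Lever is an interactable lever that notifies a linked door when the player pulls it.
; A collision component toggles an interaction flag as BP_MainCharacter enters or leaves, printing a message each time.
; When allowed, Interact fires once, calling PickUpKey on the Door reference and playing a timeline that swings the lever mesh along its roll axis.
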(event `self.Collision.OnComponentBeginOverlap`
  (params (OverlappedComponent :type "PrimitiveComponent Object Reference") (OtherActor :type "Actor Object Reference") (OtherComp :type "PrimitiveComponent Object Reference") (OtherBodyIndex :type Integer) (bFromSweep :type Boolean) (SweepResult :type "HitResult Structure (by ref)"))
  (cast `/Game/FirstPerson/MainCharacter/BP_MainCharacter` OtherActor)
  (set `self.bCanInteract` true)
  (`KismetSystemLibrary.PrintString` "You are in front of the lever"))

(event `self.Collision.OnComponentEndOverlap`
  (params (OverlappedComponent :type "PrimitiveComponent Object Reference") (OtherActor :type "Actor Object Reference") (OtherComp :type "PrimitiveComponent Object Reference") (OtherBodyIndex :type Integer))
  (cast `/Game/FirstPerson/MainCharacter/BP_MainCharacter` OtherActor)
  (set `self.bCanInteract` false)
  (`KismetSystemLibrary.PrintString` "You are no longer in front of the lever"))

(event `/Game/FirstPerson/MainCharacter/BPI_Interact.Interact`
  (if (`self.bCanInteract`)
    (`/Engine/EditorBlueprintResources/StandardMacros.DoOnce` false
      (:`Completed`
        (`/Game/DevFolder/Blueprints/Door/BPI_Door.Pick Up Key` (`self.Door`))
        (bind (_direction _lever_on) (`Timeline|Timeline`)
          (:`Update`
            (`SceneComponent.K2_SetRelativeRotation` (`self.SM_Lever`) (`KismetMathLibrary.MakeRotator` (`KismetMathLibrary.Lerp` -80.0 80.0 _lever_on)) false false)))))))

(fn `UserConstructionScript`)