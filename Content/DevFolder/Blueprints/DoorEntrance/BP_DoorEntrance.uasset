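; BP_DoorEntrance is a double entrance door that stays locked until its PickUpKey event sets the unlock flag.
; Interact, once unlocked, plays a timeline that lerps the yaw of both door meshes to swing them open.
; A box overlap shows and removes an interact widget, created at BeginPlay, for the main character.
; PickUpKey also calls NotifyUnlock after a delay, but that event is empty and its camera-change logic is unfinished and disconnected.
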(event `/Game/DevFolder/Blueprints/Door/BPI_Door.Pick Up Key`
  (set `self.bDoorUnlocked` true)
  (`KismetSystemLibrary.Delay` 2.0)
  (`self.Notify Unlock`))

(event `/Game/FirstPerson/MainCharacter/BPI_Interact.Interact`
  (if (`self.bDoorUnlocked`)
    (bind (_direction _open_time _open_time_2) (`Timeline|Door Open Timeline`)
      (:`Update`
        (`|ExecutionSequence`
          (:`then_0`
            (`SceneComponent.K2_SetRelativeRotation` (`self.SM_EntranceDoorL`) (`KismetMathLibrary.MakeRotator` 0.0 0.0 (`KismetMathLibrary.Lerp` 0.0 -90.0 _open_time)) false false))
          (:`then_1`
            (`SceneComponent.K2_SetRelativeRotation` (`self.SM_EntranceDoorR`) (`KismetMathLibrary.MakeRotator` 0.0 0.0 (`KismetMathLibrary.Lerp` -180.0 -90.0 _open_time_2)) false false)))))))

(event `Notify Unlock`
  ; Working On Camera Change
)

(event `self.ReceiveBeginPlay`
  (`|ExecutionSequence`
    (:`then_0`
      (bind _returnvalue (`|CreateWidget` "/Game/DevFolder/Widgets/WBP_Interact.WBP_Interact_C"))
      (set `self.Interact Widget Reference` _returnvalue))))

(event `self.Box.OnComponentBeginOverlap`
  (params (OverlappedComponent :type "PrimitiveComponent Object Reference") (OtherActor :type "Actor Object Reference") (OtherComp :type "PrimitiveComponent Object Reference") (OtherBodyIndex :type Integer) (bFromSweep :type Boolean) (SweepResult :type "HitResult Structure (by ref)"))
  (cast `/Game/FirstPerson/MainCharacter/BP_MainCharacter` OtherActor)
  (`UserWidget.AddToViewport` (`self.Interact Widget Reference`) 0))

(event `self.Box.OnComponentEndOverlap`
  (params (OverlappedComponent :type "PrimitiveComponent Object Reference") (OtherActor :type "Actor Object Reference") (OtherComp :type "PrimitiveComponent Object Reference") (OtherBodyIndex :type Integer))
  (cast `/Game/FirstPerson/MainCharacter/BP_MainCharacter` OtherActor)
  (`Widget.RemoveFromParent` (`self.Interact Widget Reference`)))

(fn `UserConstructionScript`)