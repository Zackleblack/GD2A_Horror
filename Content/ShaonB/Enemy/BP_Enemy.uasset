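; BP_Enemy is a wrench-wielding enemy that damages the player character and exposes a patrol route.
; AttackPlayer enables wrench overlaps during a montage; hits decrease BP_MainCharacter health, spawn force feedback and print debug lines.
; Pawn sensing sets the first AIC_Enemy found in the world to chasing, rather than specifically its own controller.
; IsInSight tests screen bounds with a delayed recheck but triggers no action, and MoveToPlayer is unconnected.
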(event `self.ReceiveBeginPlay`)

(event `self.ReceiveTick`
  (params (DeltaSeconds :type "Float (single-precision)")))

(event `Is In Sight`
  (bind (_returnvalue_x _returnvalue_y) (`KismetMathLibrary.BreakVector2D` (`WidgetLayoutLibrary.GetViewportSize`)))
  (bind _screenlocation (`PlayerController.ProjectWorldLocationToScreen` (`GameplayStatics.GetPlayerController` 0) (`SceneComponent.K2_GetComponentLocation` (`self.Mesh`)) false))
  (bind _returnvalue (and (> (`KismetMathLibrary.BreakVector2D` _screenlocation) 0.0) (> (`.Y` (`KismetMathLibrary.BreakVector2D` _screenlocation)) 0.0) (< (`KismetMathLibrary.BreakVector2D` _screenlocation) _returnvalue_x) (< (`.Y` (`KismetMathLibrary.BreakVector2D` _screenlocation)) _returnvalue_y)))
  (if (not _returnvalue)
    (`KismetSystemLibrary.Delay` 5.0)
    (if _returnvalue
      _)))

(event `AttackPlayer`
  (set `PrimitiveComponent.bGenerateOverlapEvents` true (`self.Wrench`))
  (`|PlayMontage` (`self.Mesh`)
    (:`OnCompleted`
      _)
    (:`OnInterrupted`
      _))
  (set `PrimitiveComponent.bGenerateOverlapEvents` false (`self.Wrench`))
  (`self.OnAttackEnd`))

(event `self.Wrench.OnComponentBeginOverlap`
  (params (OverlappedComponent :type "PrimitiveComponent Object Reference") (OtherActor :type "Actor Object Reference") (OtherComp :type "PrimitiveComponent Object Reference") (OtherBodyIndex :type Integer) (bFromSweep :type Boolean) (SweepResult :type "HitResult Structure (by ref)"))
  (bind _asbp_main_character (cast `/Game/FirstPerson/MainCharacter/BP_MainCharacter` OtherActor))
  (`GameplayStatics.SpawnForceFeedbackAtLocation` "/Game/ShaonB/ForceFeedback/FFE_WrenchHit.FFE_WrenchHit" (`SceneComponent.K2_GetComponentLocation` (`Character.CapsuleComponent` _asbp_main_character)) (struct) false 1.0 0.0 null)
  (`/Game/FirstPerson/BPC_Health.DecreaseHealth` (`/Game/FirstPerson/MainCharacter/BP_MainCharacter.BPC_Health` _asbp_main_character) (`self.AttackDamage`))
  (`KismetSystemLibrary.PrintString` "You've been hit by")
  (`KismetSystemLibrary.PrintString` "You've been struck by")
  (`KismetSystemLibrary.PrintString` "A smooth criminal"))

(event `self.PawnSensing.OnSeePawn`
  (params (Pawn :type "Pawn Object Reference"))
  (bind _returnvalue (`GameplayStatics.GetActorOfClass` "/Game/ShaonB/Enemy/AI/AIC_Enemy.AIC_Enemy_C"))
  (`/Game/ShaonB/Enemy/AI/AIC_Enemy.SetStateChasing` _returnvalue))

(fn `GetPatrolRoute`
  (returns (PatrolRoute :type "/Game/ShaonB/Enemy/AI/BP_PatrolRoute Object Reference"))
  (return (`self.PatrolRoute`)))

(fn `UserConstructionScript`)