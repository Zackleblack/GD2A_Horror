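; BP_Floater is a decorative actor that shows a configurable, collision-free mesh bobbing in the air.
; The construction script applies the chosen mesh, and both it and BeginPlay cache the mesh's starting relative transform.
; Tick offsets Z with a sine of time since creation and feeds a scaled rate to the Rotator component.
; That same rate is also written as the mesh's absolute relative rotation, leaving the cached starting rotation unused.
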(event `self.ReceiveBeginPlay`
  (bind _static_mesh (`self.Static Mesh`))
  (`StaticMeshComponent.SetStaticMesh` _static_mesh (`self.Mesh Input`))
  (`PrimitiveComponent.SetCollisionEnabled` _static_mesh "NoCollision")
  (set `self.Starting Location` (`SceneComponent.RelativeLocation` (`self.Static Mesh`)))
  (set `self.Starting Rotation` (`SceneComponent.RelativeRotation` (`self.Static Mesh`))))

(event `self.ReceiveTick`
  (params (DeltaSeconds :type "Float (single-precision)"))
  (bind (_starting_location_x _starting_location_y _starting_location_z) (`KismetMathLibrary.BreakVector` (`self.Starting Location`)))
  (bind _output_get (set `RotatingMovementComponent.RotationRate` (* (`self.Rotation Rate`) (`self.Rotation Speed Scale`)) (`self.Rotator`)))
  (`SceneComponent.K2_SetRelativeLocationAndRotation` (`self.Static Mesh`) (`KismetMathLibrary.MakeVector` _starting_location_x _starting_location_y (+ _starting_location_z (* (`self.Bobbing Distance`) (`KismetMathLibrary.DegSin` (* (`self.GetGameTimeSinceCreation`) (`self.Bobbing Speed`)))))) _output_get false false))

(fn `UserConstructionScript`
  (`StaticMeshComponent.SetStaticMesh` (`self.Static Mesh`) (`self.Mesh Input`))
  (set `self.Starting Location` (`SceneComponent.RelativeLocation` (`self.Static Mesh`)))
  (set `self.Starting Rotation` (`SceneComponent.RelativeRotation` (`self.Static Mesh`))))